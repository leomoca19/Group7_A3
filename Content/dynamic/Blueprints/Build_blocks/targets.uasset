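; Shootable target actor that opens the way by removing a door when its target counter runs out.
; A capsule overlap with BP_FirstPersonProjectile destroys the target, lowers its CountTargets variable by DecCount and prints the result.
; When that value equals zero, it looks up actors of the Door class and destroys the first one found.
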(event `self.Capsule.OnComponentBeginOverlap`
  (params (OverlappedComponent :type "PrimitiveComponent Object Reference") (OtherActor :type "Actor Object Reference") (OtherComp :type "PrimitiveComponent Object Reference") (OtherBodyIndex :type Integer) (bFromSweep :type Boolean) (SweepResult :type "HitResult Structure (by ref)"))
  (cast `/Game/dynamic/Blueprints/Gun/BP_FirstPersonProjectile` OtherActor)
  (`self.K2_DestroyActor`)
  (bind _output_get (set `self.countTargets` (- (`self.countTargets`) (`self.DecCount`))))
  (`KismetSystemLibrary.PrintString` (`KismetStringLibrary.Conv_IntToString` _output_get))
  (if (== (`self.countTargets`) 0)
    (bind _outactors (`GameplayStatics.GetAllActorsOfClass` "/Game/dynamic/Blueprints/Build_blocks/door.door_C"))
    (bind _asdoor (cast `/Game/dynamic/Blueprints/Build_blocks/door` (`|GetArrayItem` _outactors)))
    (`self.K2_DestroyActor` _asdoor)))

(fn `UserConstructionScript`)